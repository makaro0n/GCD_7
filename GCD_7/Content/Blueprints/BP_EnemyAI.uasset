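; BP_EnemyAI is an enemy actor that takes damage and carries a widget component, noted as an HP bar.
; Each Tick rotates the widget to face player 0's camera using a look-at rotation.
; AnyDamage subtracts from Health, prints the new value and destroys the actor at zero or below.
; The IsSeeingPlayers check on Tick has no actions, and no graph here updates the bar's value.
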(event `self.ReceiveTick`
  (params (DeltaSeconds :type "Float (single-precision)"))
  ;[1 1 1] HPBARcamera
  (`|ExecutionSequence`
    (:`then_0`
      (if (`self.is seeing players`)
        _))
    (:`then_1`
      (`SceneComponent.K2_SetWorldRotation` (`self.Widget`) (`KismetMathLibrary.FindLookAtRotation` (`SceneComponent.K2_GetComponentLocation` (`self.Widget`)) (`SceneComponent.K2_GetComponentLocation` (`PlayerCameraManager.TransformComponent` (`GameplayStatics.GetPlayerCameraManager` 0)))) false false))))

(event `self.ReceiveAnyDamage`
  (params (Damage :type "Float (single-precision)") (DamageType :type "DamageType Object Reference") (InstigatedBy :type "Controller Object Reference") (DamageCauser :type "Actor Object Reference"))
  ;[1 1 1] HP
  (set `self.Health` (- (`self.Health`) Damage))
  (`KismetSystemLibrary.PrintString` (`KismetStringLibrary.Conv_DoubleToString` (`self.Health`)))
  (if (<= (`self.Health`) 0.0)
    (`self.K2_DestroyActor`)))

(fn `UserConstructionScript`)