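; BP_VMMCharacter is a character Blueprint that sets its starting movement rotation mode and provides a test for changing animation style.
; On BeginPlay it sends itself a Movement.Rotation.Velocity gameplay event after calling the parent.
; Debug keys 1 and 2 call ServerSetAnimData, which forwards a registry ID through NetSetAnimData to the ABP_VMM anim instance via SetAnimRegistryId.
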(event `self.ReceiveBeginPlay`
  (`parent.ReceiveBeginPlay`)
  (`AbilitySystemBlueprintLibrary.SendGameplayEventToActor` self (struct :`TagName` "Movement.Rotation.Velocity")))

(event `Key|One`
  (params (Key :type "Key Structure"))
  ;[1 0 0] Change animation style - Test
  (:`Pressed`
    (`self.ServerSetAnimData` "DR_MotionAnimations:MOB1_Unarmed")))

(event `Key|Two`
  (params (Key :type "Key Structure"))
  ;[1 0 0] Change animation style - Test
  (:`Pressed`
    (`self.ServerSetAnimData` "DR_MotionAnimations:W2_Rifle")))

(event `ServerSetAnimData`
  (params (InRegistryId :type "DataRegistryId Structure"))
  ;[1 0 0] Change animation style - Test
  (`self.NetSetAnimData` InRegistryId))

(event `NetSetAnimData`
  (params (InRegistryId :type "DataRegistryId Structure"))
  ;[1 0 0] Change animation style - Test
  (bind _asabp_vmm (cast `/VirtualMotionMatching/Blueprints/Characters/ABP_VMM` (`SkeletalMeshComponent.GetAnimInstance` (`self.Mesh`))))
  (`VMM_AnimInstance.K2_SetAnimRegistryId` _asabp_vmm InRegistryId))

(fn `UserConstructionScript`)