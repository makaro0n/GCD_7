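; BP_ma_physician_01 is a citizen NPC character that reacts with fear when it sees the player attacking.
; It plays a talking montage on BeginPlay, while PawnSensing latches a flag once it sees a BP_ThirdPersonCharacter mid-attack.
; A looping timer checks that flag and replays the scare montage on each firing; nothing in these graphs clears the flag.
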(event `self.PawnSensing.OnSeePawn`
  (params (Pawn :type "Pawn Object Reference"))
  ;[1 1 1] player보임?
  (bind _asbp_third_person_character (cast `/Game/ThirdPerson/Blueprints/BP_ThirdPersonCharacter` Pawn))
  (if (`/Game/ThirdPerson/Blueprints/BP_ThirdPersonCharacter.isAttcking` _asbp_third_person_character)
    (set `self.isSeeingPlayer?` true)))

(event `self.ReceiveBeginPlay`
  ;[1 1 1] 작업부터 저항상태(선택)
  (`KismetSystemLibrary.K2_SetTimerDelegate` (delegate `Ainmturn`) 1.0 true)
  (`self.PlayAnimMontage` "/Game/Pedestrian_Convo_01/Animation/Root_Motion/sayingue4.sayingue4"))

(event `self.ReceiveTick`
  (params (DeltaSeconds :type "Float (single-precision)")))

(event `Ainmturn`
  ;[1 1 1] 작업부터 저항상태(선택)
  (if (`self.isSeeingPlayer?`)
    (`self.PlayAnimMontage` "/Game/Scared_01/Animation/Root_Motion/scareloopue4.scareloopue4")))

(fn `UserConstructionScript`
  (`parent.UserConstructionScript`))